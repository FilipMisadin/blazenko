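; Cipal is a sword-and-shield melee AI enemy that fights the player in waves.
; On spawn it attaches sword and shield actors to mesh sockets.
; Player sword overlaps are blocked in shield mode unless stunned, otherwise they cut health and update its bar; death decrements the player's enemy count, spawning the next wave at zero.
; Combo delay, block-break and pushback events toggle Blackboard flags to pause its behavior.
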(event `self.ReceiveBeginPlay`
  (bind _mesh (`self.Mesh`))
  (bind _mesh_2 (`self.Mesh`))
  (`parent.ReceiveBeginPlay`)
  (bind _returnvalue (`|SpawnActorFromClass` "/Game/ThirdPersonBP/Models/Sword/SrdelaSwordBP.SrdelaSwordBP_C" (`SceneComponent.GetSocketTransform` _mesh "SwordSocket" "RTS_World") "Undefined" "OverrideRootScale" null null))
  (set `/Game/ThirdPersonBP/Models/Sword/SrdelaSwordBP.AIHoldingSword` self _returnvalue)
  (bind _output_get (set `self.SwordInstance` _returnvalue))
  (`self.K2_AttachToComponent` _output_get _mesh "SwordSocket" "SnapToTarget" "SnapToTarget" "SnapToTarget" true)
  (bind _returnvalue_2 (`|SpawnActorFromClass` "/Game/AI/Cipal/Shield/EnemyShieldBP.EnemyShieldBP_C" (`SceneComponent.GetSocketTransform` _mesh_2 "ShieldSocket" "RTS_World") "Undefined" "OverrideRootScale" null null))
  (set `/Game/AI/Cipal/Shield/EnemyShieldBP.AIHoldingShield` self _returnvalue_2)
  (bind _output_get_2 (set `self.ShieldInstance` _returnvalue_2))
  (`self.K2_AttachToComponent` _output_get_2 _mesh_2 "ShieldSocket" "SnapToTarget" "SnapToTarget" "SnapToTarget" true)
  (set `self.Health` 100)
  (set `self.Damage` 20))

(event `ComboDelay`
  (`KismetSystemLibrary.RetriggerableDelay` 1.5)
  (`BlackboardComponent.SetValueAsBool` (`AIBlueprintHelperLibrary.GetBlackboard` self) "ComboWait" false))

(event `StopAllActions`
  (params (Duration :type "Float (double-precision)"))
  (bind _returnvalue (`AIBlueprintHelperLibrary.GetBlackboard` self))
  (`KismetSystemLibrary.PrintString` "STOP ALL ACTIONS true in blueprint" false)
  (`BlackboardComponent.SetValueAsBool` _returnvalue "StopAllActions" true)
  (`|PlayMontage` (`self.Mesh`) "/Game/AI/Cipal/Character/Cipal_BlockBreak.Cipal_BlockBreak"
    (:`then`
      (`BlackboardComponent.SetValueAsBool` _returnvalue "ComboWait" true)
      (`BlackboardComponent.SetValueAsBool` _returnvalue "ChainCombo" false)
      (`AIBlueprintHelperLibrary.SimpleMoveToLocation` (`self.GetController` self) (+ (`self.K2_GetActorLocation`) (* (`KismetMathLibrary.GetRightVector` (`self.K2_GetActorRotation` (`/Game/ThirdPersonBP/Blueprints/ThirdPersonCharacter.ShieldInstance` (cast `/Game/ThirdPersonBP/Blueprints/ThirdPersonCharacter` (`GameplayStatics.GetPlayerCharacter` 0) :!pure true)))) 150.0)))
      (`KismetSystemLibrary.RetriggerableDelay` Duration)
      (`BlackboardComponent.SetValueAsBool` _returnvalue "ComboWait" false)
      (`BlackboardComponent.SetValueAsBool` _returnvalue "StopAllActions" false)
      (`KismetSystemLibrary.PrintString` "STOP ALL ACTIONS false in blueprint" false))))

(event `DestroyActor`
  (`self.K2_DestroyActor` (`self.SwordInstance`))
  (`self.K2_DestroyActor` (`self.ShieldInstance`))
  (`self.K2_DestroyActor`))

(event `self.CapsuleComponent.OnComponentBeginOverlap`
  (params (OverlappedComponent :type "PrimitiveComponent Object Reference") (OtherActor :type "Actor Object Reference") (OtherComp :type "PrimitiveComponent Object Reference") (OtherBodyIndex :type Integer) (bFromSweep :type Boolean) (SweepResult :type "HitResult Structure (by ref)"))
  (bind _health (`self.Health`))
  (cast `/Game/ThirdPersonBP/Models/Sword/SrdelaSwordBP` OtherActor)
  (if (`/Game/ThirdPersonBP/Blueprints/ThirdPersonCharacter.IsAttacking` (cast `/Game/ThirdPersonBP/Blueprints/ThirdPersonCharacter` (`GameplayStatics.GetPlayerPawn` 0) :!pure true))
    (if (and (`self.ShieldUpMode`) (not (`BlackboardComponent.GetValueAsBool` (`AIBlueprintHelperLibrary.GetBlackboard` self) "StopAllActions")))
      (`GameplayStatics.PlaySoundAtLocation` "/Game/Audio/Shield/SwordOnShieldHit.SwordOnShieldHit" (`self.K2_GetActorLocation` (`self.ShieldInstance`)) (struct) 1.0 1.0 0.0 null null null)
      (`self.PlayAnimMontage` "/Game/AI/Cipal/Character/Cipal_BlockHit.Cipal_BlockHit")
      (else
        (set `self.Health` (- _health 50))
        (if (<= _health 0)
          (`/Game/ThirdPersonBP/Blueprints/ThirdPersonCharacter.StaminaGainED` (cast `/Game/ThirdPersonBP/Blueprints/ThirdPersonCharacter` (`GameplayStatics.GetPlayerPawn` 0) :!pure true))
          (`self.HandleDeath`)
          (else
            (bind _ashealth_widget (cast `/Game/HUD/HealthWidget` (`WidgetComponent.GetUserWidgetObject` (`self.HealthWidget`))))
            (`ProgressBar.SetPercent` (`/Game/HUD/HealthWidget.HealthBar` _ashealth_widget) (/ (`KismetMathLibrary.Conv_IntToDouble` (`self.Health`)) 100.0))))))))

(event `HandleDeath`
  (bind _asthird_person_character (cast `/Game/ThirdPersonBP/Blueprints/ThirdPersonCharacter` (`GameplayStatics.GetPlayerPawn` 0) :!pure true))
  (`self.K2_DestroyActor` (`self.SwordInstance`))
  (`self.K2_DestroyActor` (`self.ShieldInstance`))
  (`self.K2_DestroyActor`)
  (bind _output_get (set `/Game/ThirdPersonBP/Blueprints/ThirdPersonCharacter.NumberOfAIsInLevel` (- (`/Game/ThirdPersonBP/Blueprints/ThirdPersonCharacter.NumberOfAIsInLevel` _asthird_person_character) 1) _asthird_person_character))
  (if (== _output_get 0)
    (`/Game/ThirdPersonBP/Blueprints/ThirdPersonCharacter.SpawnWave` _asthird_person_character)))

(event `PushedBack`
  (params (Delay :type "Float (double-precision)"))
  (bind _returnvalue (`AIBlueprintHelperLibrary.GetBlackboard` self))
  (`KismetSystemLibrary.RetriggerableDelay` Delay)
  (`BlackboardComponent.SetValueAsBool` _returnvalue "StopAllActions" true)
  (`|PlayMontage` (`self.Mesh`) "/Game/AI/Cipal/Character/Cipal_BlockBreak.Cipal_BlockBreak"
    (:`OnCompleted`
      _)
    (:`OnInterrupted`
      _))
  (`BlackboardComponent.SetValueAsBool` _returnvalue "StopAllActions" false)
  (`KismetSystemLibrary.PrintString` "STUN OVER"))

(fn `UserConstructionScript`
  (`parent.UserConstructionScript`))