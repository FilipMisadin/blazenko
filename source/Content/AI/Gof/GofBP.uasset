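; Gof is a hammer-wielding enemy AI that attaches a spawned HammerBP to its hand socket and sets its own health, damage and walk speed.
; Capsule overlaps with the player's sword during attacks reduce health and update its health bar.
; Death destroys it and its weapons, decrements the player's AI count and triggers the next wave at zero.
; ComboDelay clears a blackboard wait flag; StopAllActions is empty, its block-break logic left disconnected.
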(event `self.ReceiveBeginPlay`
  (bind _mesh (`self.Mesh`))
  (`parent.ReceiveBeginPlay`)
  (bind _returnvalue (`|SpawnActorFromClass` "/Game/AI/Gof/Models/Hammer/HammerBP.HammerBP_C" (`SceneComponent.GetSocketTransform` _mesh "SwordSocket" "RTS_World") "Undefined" "OverrideRootScale" null null))
  (set `/Game/AI/Gof/Models/Hammer/HammerBP.AIHoldingHammer` self _returnvalue)
  (bind _output_get (set `self.HammerInstance` _returnvalue))
  (`self.K2_AttachToComponent` _output_get _mesh "SwordSocket" "SnapToTarget" "SnapToTarget" "SnapToTarget" true)
  (set `self.Health` 250)
  (set `self.Damage` 60)
  (set `CharacterMovementComponent.MaxWalkSpeed` 200.0 (`self.CharacterMovement`)))

(event `ComboDelay`
  (`KismetSystemLibrary.RetriggerableDelay` 1.5)
  (`BlackboardComponent.SetValueAsBool` (`AIBlueprintHelperLibrary.GetBlackboard` self) "ComboWait" false))

(event `StopAllActions`
  (params (Duration :type "Float (double-precision)")))

(event `DestroyActor`
  (`self.K2_DestroyActor` (`self.HammerInstance`))
  (`self.K2_DestroyActor`))

(event `self.Footstep`
  (`|MultiGate` false true
    (:`Out 0`
      (`GameplayStatics.PlaySound2D` "/Game/Audio/Footsteps/footstep_dirt_1.footstep_dirt_1" 1.0 1.0 0.0 null null))
    (:`Out 1`
      (`GameplayStatics.PlaySound2D` "/Game/Audio/Footsteps/footstep_dirt_2.footstep_dirt_2" 1.0 1.0 0.0 null null))))

(event `self.CapsuleComponent.OnComponentBeginOverlap`
  (params (OverlappedComponent :type "PrimitiveComponent Object Reference") (OtherActor :type "Actor Object Reference") (OtherComp :type "PrimitiveComponent Object Reference") (OtherBodyIndex :type Integer) (bFromSweep :type Boolean) (SweepResult :type "HitResult Structure (by ref)"))
  (bind _health (`self.Health`))
  (cast `/Game/ThirdPersonBP/Models/Sword/SrdelaSwordBP` OtherActor)
  (if (`/Game/ThirdPersonBP/Blueprints/ThirdPersonCharacter.IsAttacking` (cast `/Game/ThirdPersonBP/Blueprints/ThirdPersonCharacter` (`GameplayStatics.GetPlayerPawn` 0) :!pure true))
    (set `self.Health` (- _health 50))
    (if (<= _health 0)
      (`self.HandleDeath`)
      (`self.K2_DestroyActor` (`self.HammerInstance`))
      (else
        (bind _ashealth_widget (cast `/Game/HUD/HealthWidget` (`WidgetComponent.GetUserWidgetObject` (`self.HealthWidget`))))
        (`ProgressBar.SetPercent` (`/Game/HUD/HealthWidget.HealthBar` _ashealth_widget) (/ (`KismetMathLibrary.Conv_IntToDouble` (`self.Health`)) 250.0))))))

(event `HandleDeath`
  (bind _asthird_person_character (cast `/Game/ThirdPersonBP/Blueprints/ThirdPersonCharacter` (`GameplayStatics.GetPlayerPawn` 0) :!pure true))
  (`self.K2_DestroyActor` (`self.SwordInstance`))
  (`self.K2_DestroyActor` (`self.ShieldInstance`))
  (`self.K2_DestroyActor`)
  (bind _output_get (set `/Game/ThirdPersonBP/Blueprints/ThirdPersonCharacter.NumberOfAIsInLevel` (- (`/Game/ThirdPersonBP/Blueprints/ThirdPersonCharacter.NumberOfAIsInLevel` _asthird_person_character) 1) _asthird_person_character))
  (if (== _output_get 0)
    (`/Game/ThirdPersonBP/Blueprints/ThirdPersonCharacter.SpawnWave` _asthird_person_character)))

(fn `UserConstructionScript`)