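; DemoBellBP is a bell actor that triggers the player character's demo mode when struck with the sword.
; It loops a silent animation until an SrdelaSwordBP overlaps it while the player's ThirdPersonCharacter is attacking.
; A one-time hit flag then guards the call to StartDemoMODE, a ring sound and a looping ding animation, and the bell destroys itself after a short delay.
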(event `self.ReceiveBeginPlay`
  (`SkeletalMeshComponent.PlayAnimation` (`self.Bell`) "/Game/MapModels/Bell/DemoBell_Anim_DemoBellBone_BellSilence.DemoBell_Anim_DemoBellBone_BellSilence" true))

(event `self.ReceiveActorBeginOverlap`
  (params (OtherActor :type "Actor Object Reference"))
  (bind _asthird_person_character (cast `/Game/ThirdPersonBP/Blueprints/ThirdPersonCharacter` (`GameplayStatics.GetPlayerPawn` 0) :!pure true))
  (if (not (`self.AlreadyHit`))
    (cast `/Game/ThirdPersonBP/Models/Sword/SrdelaSwordBP` OtherActor)
    (if (`/Game/ThirdPersonBP/Blueprints/ThirdPersonCharacter.IsAttacking` _asthird_person_character)
      (set `self.AlreadyHit` true)
      (`/Game/ThirdPersonBP/Blueprints/ThirdPersonCharacter.StartDemoMODE` _asthird_person_character)
      (`GameplayStatics.PlaySound2D` "/Game/MapModels/Bell/Blastwave_FX_BoxingBellRing_S08SP_136.Blastwave_FX_BoxingBellRing_S08SP_136" 1.0 1.0 0.0 null null)
      (`SkeletalMeshComponent.PlayAnimation` (`self.Bell`) "/Game/MapModels/Bell/DemoBell_Anim_DemoBellBone_BellDING.DemoBell_Anim_DemoBellBone_BellDING" true)
      (`KismetSystemLibrary.RetriggerableDelay` 5.0)
      (`self.K2_DestroyActor`))))

(fn `UserConstructionScript`)